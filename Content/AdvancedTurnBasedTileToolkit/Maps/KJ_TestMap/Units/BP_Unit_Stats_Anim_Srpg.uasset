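; Turn-based tile toolkit unit for an SRPG test map, where each unit is a stack with shared health.
; DefaultAttack rolls crits, fires pre/post dispatcher events, queues the attack action and applies damage.
; CalculateAttackDamage scales random damage by stack count and crit, computing but not applying an attack-versus-defense modifier.
; ModifyHealth shows splash text and converts lethal damage into lost stack members, carrying the remainder into health.
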(fn `CalculateAttackDamage`
  (params (Target :type "Actor Object Reference") (bCriticalHit :type Boolean))
  (returns (Damage :type Integer))
  (locals (LocalDamageModifier :type "Float (double-precision)" :default 0.0))
  (bind (_bhasstat _value) (message `/Game/AdvancedTurnBasedTileToolkit/Maps/Experimental/StatSystem/Core/BPI_Stats.GetStatValue` (`local.Target`) (struct :`TagName` "Stat.Defense")))
  (bind (_bhasstat_2 _value_2) (`self.GetStatValue` (struct :`TagName` "Stat.Attack")))
  (bind _returnvalue (- _value_2 _value))
  (set `local.LocalDamageModifier` (`KismetMathLibrary.FClamp` (+ (select `bool` (> _returnvalue 0.0) :`false` (* _returnvalue 0.025) :`true` (* _returnvalue 0.05)) 1.0) 0.7 3.0))
  (bind (_bhasstat_3 _value_3) (`self.GetStatValue` (struct :`TagName` "Stat.CritDamage")))
  (bind (_bhasstat_4 _value_4) (`self.GetStatValue` (struct :`TagName` "Stat.RandomDamage")))
  (bind (_bhasstat_5 _value_5) (`self.GetStatValue` (struct :`TagName` "Stat.Damage")))
  (bind (_bhasstat_6 _value_6) (`self.GetStatValue` (struct :`TagName` "Stat.Stack")))
  (return (`KismetMathLibrary.FTrunc` (* _value_6 (* (`KismetMathLibrary.RandomFloatInRange` _value_5 (+ _value_5 _value_4)) (`KismetMathLibrary.SelectFloat` (/ _value_3 100.0) 1.0 (`local.bCriticalHit`)))))))

(fn `DefaultAttack`
  (params (TargetUnit :type "/Game/AdvancedTurnBasedTileToolkit/Core/Units/BP_Unit Object Reference (by ref)"))
  (returns (bSuccess :type Boolean))
  (locals (bLocalCrit :type Boolean :default false))
  (bind (_bhasstat _value) (`self.GetStatValue` (struct :`TagName` "Stat.Crit")))
  (set `local.bLocalCrit` (> _value (`KismetMathLibrary.RandomFloatInRange` 0.0 100.0)))
  (`/Game/AdvancedTurnBasedTileToolkit/Maps/Experimental/StatSystem/Core/BP_DispatcherHubComponent.CallEventWithPayload` (`self.BP_DispatcherHubComponent`) (struct :`TagName` "Event.UnitAttackingPre") self null true (`local.TargetUnit`))
  (`/Game/AdvancedTurnBasedTileToolkit/Maps/Experimental/StatSystem/Core/BP_DispatcherHubComponent.CallEvent` (`self.GetComponentByClass` (`local.TargetUnit`) "/Game/AdvancedTurnBasedTileToolkit/Maps/Experimental/StatSystem/Core/BP_DispatcherHubComponent.BP_DispatcherHubComponent_C") (struct :`TagName` "Event.UnitAttackedPre") self null true)
  (`self.QueueAttackAction` (`local.TargetUnit`) (> (`/Game/AdvancedTurnBasedTileToolkit/Core/Grid/BP_GridManager.FindDistanceIinTilesBetweenIndexes` (`self.GridManagerRef`) (`self.GridIndex`) (`/Game/AdvancedTurnBasedTileToolkit/Core/Units/BP_Unit.GridIndex` (`local.TargetUnit`)) false) 1))
  (if (`local.bLocalCrit`)
    (bind _puppet (message `/Game/AdvancedTurnBasedTileToolkit/Core/BPI_Initiative.GetPuppet` (`local.TargetUnit`)))
    (`|SpawnActorFromClass` "/Game/AdvancedTurnBasedTileToolkit/Maps/Experimental/StatSystem/Actions/BP_Action_SplashTextOnComponent.BP_Action_SplashTextOnComponent_C" (`KismetMathLibrary.MakeTransform` (0.0 0.0 0.0)) "AlwaysSpawn" "OverrideRootScale" null "CRITICAL" (struct :`R` 1.0 :`A` 1.0) (`self.GetComponentByClass` _puppet "/Game/AdvancedTurnBasedTileToolkit/Maps/Experimental/StatSystem/Core/BP_StatSplashComponent.BP_StatSplashComponent_C") -1.0 "NewEnumerator0" null))
  (bind _damage (`self.CalculateAttackDamage` (`local.TargetUnit`) (`local.bLocalCrit`)))
  (`self.ModifyHealth` (`local.TargetUnit`) (* (`KismetMathLibrary.Conv_IntToDouble` _damage) -1.0) true (`self.PostHitDelay`))
  (`/Game/AdvancedTurnBasedTileToolkit/Maps/Experimental/StatSystem/Core/BP_DispatcherHubComponent.CallEventWithPayload` (`self.BP_DispatcherHubComponent`) (struct :`TagName` "Event.UnitAttackingPost") self null true (`local.TargetUnit`))
  (bind _targetunit (`local.TargetUnit`)
    (:`then`
      (`/Game/AdvancedTurnBasedTileToolkit/Maps/Experimental/StatSystem/Core/BP_DispatcherHubComponent.CallEvent` (`self.GetComponentByClass` _targetunit "/Game/AdvancedTurnBasedTileToolkit/Maps/Experimental/StatSystem/Core/BP_DispatcherHubComponent.BP_DispatcherHubComponent_C") (struct :`TagName` "Event.UnitAttackedPost") self null true)
      (return true))
    (:`else`
      (return true))))

(fn `ModifyHealth`
  (params (Change :type "Float (double-precision)") (bAutoAnimate :type Boolean) (EndDelay :type "Float (double-precision)"))
  (locals (LocalOldHealth :type "Float (double-precision)" :default 0.0) (LocalMaxHealth :type "Float (double-precision)" :default 0.0) (LocalNewHealth :type "Float (double-precision)" :default 0.0))
  (bind _localmaxhealth (`local.LocalMaxHealth`))
  (bind _returnvalue (`KismetMathLibrary.Abs` (+ (`local.LocalOldHealth`) (`local.Change`))))
  (`|SpawnActorFromClass` "/Game/AdvancedTurnBasedTileToolkit/Maps/Experimental/StatSystem/Actions/BP_Action_SplashTextOnComponent.BP_Action_SplashTextOnComponent_C" (`KismetMathLibrary.MakeTransform` (0.0 0.0 0.0)) "AlwaysSpawn" "OverrideRootScale" null (`KismetTextLibrary.Conv_DoubleToText` (`KismetMathLibrary.Abs` (`local.Change`)) "HalfToEven") (struct :`R` 1.0 :`A` 1.0) (`self.GetComponentByClass` (`self.Puppet`) "/Game/AdvancedTurnBasedTileToolkit/Maps/Experimental/StatSystem/Core/BP_StatSplashComponent.BP_StatSplashComponent_C") -1.0 "NewEnumerator0" null)
  (bind (_bhasstat _value) (`self.GetStatValue` (struct :`TagName` "Stat.Health")))
  (set `local.LocalOldHealth` _value)
  (if (or (> (`local.Change`) 0.0) (> (+ (`local.LocalOldHealth`) (`local.Change`)) 0.0))
    (`parent.ModifyHealth` (`local.Change`) (`local.bAutoAnimate`) (`local.EndDelay`))
    (else
      (bind (_bsuccess _maxvalue) (`self.GetStatMaxValue` (struct :`TagName` "Stat.Health")))
      (set `local.LocalMaxHealth` _maxvalue)
      (`self.SetStatToValue` (struct :`TagName` "Stat.Stack") (`KismetMathLibrary.Conv_IntToDouble` (`KismetMathLibrary.Max` (- (`KismetMathLibrary.FTrunc` (`.Value` (`self.GetStatValuePure` (struct :`TagName` "Stat.Stack")))) (+ (`KismetMathLibrary.FCeil` (/ _returnvalue _localmaxhealth)) (`KismetMathLibrary.Conv_BoolToInt` (== (mod _returnvalue _localmaxhealth) 0.0)))))))
      (bind _output_get (set `local.LocalNewHealth` (`KismetMathLibrary.SelectFloat` 0.0 (- (`local.LocalMaxHealth`) (mod (`KismetMathLibrary.Abs` (+ (`local.LocalOldHealth`) (`local.Change`))) (`local.LocalMaxHealth`))) (== (`.Value` (`self.GetStatValuePure` (struct :`TagName` "Stat.Stack"))) 0.0))))
      (if (not (< _output_get (`local.LocalOldHealth`)))
        (`|SpawnActorFromClass` "/Game/AdvancedTurnBasedTileToolkit/Core/Actions/BP_Action_AnimatePuppet.BP_Action_AnimatePuppet_C" (`KismetMathLibrary.MakeTransform` (0.0 0.0 0.0)) "AlwaysSpawn" "OverrideRootScale" null (`self.Puppet`) (struct :`TagName` "Anim.Hurt") false -1.0 "NewEnumerator0" null))
      (`self.SetStatToValue` (struct :`TagName` "Stat.Health") (`local.LocalNewHealth`))
      (return))))

(fn `UserConstructionScript`
  (`parent.UserConstructionScript`))